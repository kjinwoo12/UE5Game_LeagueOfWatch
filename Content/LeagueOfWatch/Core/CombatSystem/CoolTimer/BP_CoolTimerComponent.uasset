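; BP_CoolTimerComponent is a cooldown timer component in the combat system that tracks one remaining cooldown and signals when it ends.
; Start sets the remaining time, overwriting any current value, and Tick subtracts delta seconds while it is above zero.
; When the countdown reaches zero or below, it fires the OnCoolTimeDone dispatcher.
; IsOnCool and IsOffCool report whether the cooldown is still running.
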(event Custom|Start
  (params (CoolTime :type Float%20%28double-precision%29))
  (Variables|Default|SetCurrentCoolTime CoolTime))

(event EventBeginPlay)

(event EventTick
  (params (DeltaSeconds :type Float%20%28single-precision%29))
  (if (> (Variables|Default|GetCurrentCoolTime) 0.0)
    (Variables|Default|SetCurrentCoolTime (- (Variables|Default|GetCurrentCoolTime) DeltaSeconds))
    (if (<= (Variables|Default|GetCurrentCoolTime) 0.0)
      (Default|CallOnCoolTimeDone))))

(fn IsonCool
  (return (> (Variables|Default|GetCurrentCoolTime) 0.0)))

(fn IsOffCool
  (return (<= (Variables|Default|GetCurrentCoolTime) 0.0)))