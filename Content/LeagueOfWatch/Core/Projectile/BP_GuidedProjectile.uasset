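; Guided projectile that homes on a Target actor and deals attack damage when it reaches it.
; Each tick it caches the Target's location before running the parent tick, and GetGoal returns that cached point, so the last known position remains if the Target becomes invalid.
; Overlapping the valid Target triggers OnHitTarget, which applies Damage, then destroys the projectile; other overlaps are ignored.
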(event Custom|OnHitTarget
  (params (Target :type Actor%20Object%20Reference))
  (Game|Damage|ApplyDamage Target (Variables|파라미터|GetDamage) 0 0 "/Game/LeagueOfWatch/Core/CombatSystem/DamageTypes/BP_DamageType_AttackDamage.BP_DamageType_AttackDamage_C"))

(event EventBeginPlay
  (bind _target (Variables|Param|GetTarget))
  (Utilities|IsValid _target
    (:Is%20Valid
      (Variables|Default|SetTargetLastLocation (Transformation|GetActorLocation _target)))))

(event Collision|EventActorBeginOverlap
  (params (OtherActor :type Actor%20Object%20Reference))
  (bind _target (Variables|Param|GetTarget))
  (if (and (Utilities|IsValid _target) (== _target OtherActor))
    (CallFunction|OnHitTarget OtherActor)
    (Actor|DestroyActor)))

(event EventTick
  (params (DeltaSeconds :type Float%20%28single-precision%29))
  (bind _target (Variables|Param|GetTarget))
  (Utilities|IsValid _target
    (:Is%20Valid
      (Variables|Default|SetTargetLastLocation (Transformation|GetActorLocation _target)))
    (:Is%20Not%20Valid
      _))
  (|CallParentFunction DeltaSeconds))

(fn ConstructionScript
  (|CallParentFunction))

(fn GetGoal
  (return (Variables|Default|GetTargetLastLocation)))