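; Weapon instance Blueprint that drives character animation when the weapon is equipped or unequipped.
; On equip it caches the equipment component's mesh and gameplay tags, then uses those tags to select an animation layer class.
; A shared helper links that layer to the mesh and plays the paired montage, forwarding its callbacks.
; Unequip repeats this and clears the mesh reference without waiting for completion; DetermineCosmeticTags is an empty stub.
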(event EventOnEquippedEvent
  (params (EquipmentComponent :type Equipment%20Component%20Object%20Reference))
  (Variables|애니메이션|SetAnimatedMeshComponent (Variables|/Script/EquipmentLibrary.EquipmentComponent|GetMesh EquipmentComponent))
  (bind _output_get (Variables|Default|SetGameplayTagContainer (Variables|/Script/EquipmentLibrary.EquipmentComponent|GetGameplayTagContainer EquipmentComponent)))
  (Utilities|ActivateAnimLayerandPlayPairedAnim (Class|LeagueEquipmentInstance|GetEquippedAnimInstance _output_get) (Variables|애니메이션|GetEquipMontage)))

(event EventOnUnequippedEvent
  (Utilities|ActivateAnimLayerandPlayPairedAnim (Class|LeagueEquipmentInstance|GetUnequippedAnimInstance (Variables|Default|GetGameplayTagContainer)) (Variables|애니메이션|GetUnequipMontage)
    (:then
      (Variables|애니메이션|SetAnimatedMeshComponent 0))))

(fn DetermineCosmeticTags)