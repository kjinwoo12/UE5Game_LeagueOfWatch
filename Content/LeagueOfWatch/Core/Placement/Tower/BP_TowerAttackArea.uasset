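; BP_TowerAttackArea is the detection area that tracks which actors a tower can attack.
; On begin overlap it adds actors tagged TowerAttackTarget whose team, read through GetTeamMessage, differs from its own Team.
; On end overlap it removes the actor from AttackTargets.
; Each add or successful removal broadcasts the list through the OnUpdaetAttackTargets dispatcher, so listeners receive changes without polling.
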(event EventBeginPlay)

(event EventTick
  (params (DeltaSeconds :type Float%20%28single-precision%29)))

(event Collision|EventActorBeginOverlap
  (params (OtherActor :type Actor%20Object%20Reference))
  (bind _team (Class|BPITeamSystem|GetTeam(Message) OtherActor))
  (if (and (Utilities|Enum|NotEqual(Enum) _team (Variables|Default|GetTeam)) (Actor|ActorHasTag OtherActor "TowerAttackTarget"))
    (Utilities|Array|Add (Variables|Default|GetAttackTargets) OtherActor)
    (Default|CallOnUpdaetAttackTargets (Variables|Default|GetAttackTargets))))

(event Collision|EventActorEndOverlap
  (params (OtherActor :type Actor%20Object%20Reference))
  (bind _returnvalue (Utilities|Array|RemoveItem (Variables|Default|GetAttackTargets) OtherActor))
  (if _returnvalue
    (Default|CallOnUpdaetAttackTargets (Variables|Default|GetAttackTargets))))

(fn ConstructionScript)