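; Player controller for the character selection level that coordinates player readiness, character picks and leaving the match.
; It relays game state, player state and all-ready events to every actor implementing BPI_CharacterSelectionEventListener.
; It counts begun player states and tells the server it is ready once the count matches the PlayerArray.
; Selection and confirmation go through server RPCs to the PlayerState and GameMode, while client RPCs announce all-ready and open the Entry level.
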(event Custom|OnGameStateBegin
  (params (GameState :type BP%20Game%20State%20Character%20Selection%20Object%20Reference))
  (bind _output_get (Variables|Default|SetBP%20Game%20State%20Character%20Selection GameState))
  (bind _outactors (Actor|GetAllActorswithInterface "/Game/LeagueOfWatch/Core/GameModes/DependOnLevel/CharacterSelection/BPI_CharacterSelectionEventListener.BPI_CharacterSelectionEventListener_C"))
  (for _array_element _outactors
    (Class|BPICharacterSelectionEventListener|OnGameStateBegin(Message) _array_element _output_get)))

(event Custom|Server%20RPC%20On%20Character%20Selected
  (params (SelectedCharacterInfo :type S%20Playable%20Character%20Info%20Structure))
  (bind _asbp_player_state_character_selection (Utilities|Casting|CastToBP_PlayerState_CharacterSelection (Variables|GetPlayerState)))
  (if (not (Variables|/Game/LeagueOfWatch/Core/GameModes/DependOnLevel/CharacterSelection/BP_PlayerState_CharacterSelection.BP_PlayerState_CharacterSelection_C|GetIsCharacterConfirmed _asbp_player_state_character_selection))
    (Variables|/Game/LeagueOfWatch/Core/GameModes/DependOnLevel/CharacterSelection/BP_PlayerState_CharacterSelection.BP_PlayerState_CharacterSelection_C|SetSelectedCharacter _asbp_player_state_character_selection SelectedCharacterInfo)))

(event Custom|LeaveServer
  (CallFunction|ClientRPCLeaveServer))

(event Custom|Client%20RPC%20Leave%20%20Server
  (Game|OpenLevel(byObjectReference) "/Game/LeagueOfWatch/Maps/Entry.Entry"))

(event Custom|OnLocalPlayerStateBegin
  (params (PlayerState :type BP%20Player%20State%20Character%20Selection%20Object%20Reference))
  (bind _bp_game_state_character_selection (Variables|Default|GetBP%20Game%20State%20Character%20Selection))
  (Development|PrintString "BP_PlayerController_CharacterSelection - OnLocalPlayerStateBegin" true true "(R=0.000000,G=0.660000,B=1.000000,A=1.000000)" 2e+01)
  (bind _outactors (Actor|GetAllActorswithInterface "/Game/LeagueOfWatch/Core/GameModes/DependOnLevel/CharacterSelection/BPI_CharacterSelectionEventListener.BPI_CharacterSelectionEventListener_C"))
  (for _array_element _outactors
    (Class|BPICharacterSelectionEventListener|OnLocalPlayerStateBegin(Message) _array_element PlayerState))
  (bind _result (Math|Integer|IncrementInt (Variables|Default|GetPlayerStateNum))
    (:%20%20
      (if (Utilities|IsValid _bp_game_state_character_selection)
        (if (== _result (Utilities|Array|Length (Variables|/Script/Engine.GameStateBase|GetPlayerArray _bp_game_state_character_selection)))
          (CallFunction|ServerRPCPlayerReady))))))

(event Custom|On%20All%20Players%20Ready
  (CallFunction|ClientRPConAllPlayersConnected)
  (bind _outactors (Actor|GetAllActorswithInterface "/Game/LeagueOfWatch/Core/GameModes/DependOnLevel/CharacterSelection/BPI_CharacterSelectionEventListener.BPI_CharacterSelectionEventListener_C"))
  (for _array_element _outactors
    (Class|BPICharacterSelectionEventListener|OnAllPlayersReady(Message) _array_element)))

(event Custom|Client%20RPC%20On%20All%20Players%20Connected
  (bind _outactors (Actor|GetAllActorswithInterface "/Game/LeagueOfWatch/Core/GameModes/DependOnLevel/CharacterSelection/BPI_CharacterSelectionEventListener.BPI_CharacterSelectionEventListener_C"))
  (for _array_element _outactors
    (Class|BPICharacterSelectionEventListener|OnAllPlayersReady(Message) _array_element)))

(event Custom|Server%20RPC%20Player%20Ready
  (bind _asbp_game_mode_character_selection (Utilities|Casting|CastToBP_GameMode_CharacterSelection (Game|GetGameMode)))
  (Default|OnPlayerReady _asbp_game_mode_character_selection self))

(event Custom|OnPlayerStateBegin
  (params (PlayerState :type BP%20Player%20State%20Character%20Selection%20Object%20Reference))
  (bind _bp_game_state_character_selection (Variables|Default|GetBP%20Game%20State%20Character%20Selection))
  (bind _outactors (Actor|GetAllActorswithInterface "/Game/LeagueOfWatch/Core/GameModes/DependOnLevel/CharacterSelection/BPI_CharacterSelectionEventListener.BPI_CharacterSelectionEventListener_C"))
  (for _array_element _outactors
    (Class|BPICharacterSelectionEventListener|OnPlayerStateBegin(Message) _array_element PlayerState))
  (bind _result (Math|Integer|IncrementInt (Variables|Default|GetPlayerStateNum))
    (:%20%20
      (if (Utilities|IsValid _bp_game_state_character_selection)
        (if (== _result (Utilities|Array|Length (Variables|/Script/Engine.GameStateBase|GetPlayerArray _bp_game_state_character_selection)))
          (CallFunction|ServerRPCPlayerReady))))))

(event Custom|Server%20RPC%20On%20Character%20Confirmed
  (bind _asbp_game_mode_character_selection (Utilities|Casting|CastToBP_GameMode_CharacterSelection (Game|GetGameMode)))
  (Default|OnCharacterConfirmed _asbp_game_mode_character_selection self))

(event EventBeginPlay)

(event EventTick
  (params (DeltaSeconds :type Float%20%28single-precision%29)))

(event EventOnCharacterSelected
  (params (SelectedCharacterInfo :type S%20Playable%20Character%20Info%20Structure))
  (CallFunction|ServerRPConCharacterSelected SelectedCharacterInfo))

(event EventOnCharacterConfirmed
  (CallFunction|ServerRPConCharacterConfirmed))

(fn ConstructionScript)