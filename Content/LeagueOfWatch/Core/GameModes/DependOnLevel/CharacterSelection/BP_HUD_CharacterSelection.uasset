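; HUD for the character selection level that creates the main character selection widget and adds it to the viewport on BeginPlay.
; It relays game state begin, local and other player state begin, and all-players-ready events to the UI.
; Each event finds every widget implementing BPI_CharacterSelectionEventListener, nested ones included, and calls the matching interface message, so widgets need no direct references from the HUD.
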(event EventBeginPlay
  (bind _returnvalue (UserInterface|CreateWidget "/Game/LeagueOfWatch/Widgets/DependOnLevel/CharacterSelection/WBP_CharacterSelection_Main.WBP_CharacterSelection_Main_C"))
  (UserInterface|Viewport|AddtoViewport _returnvalue 0))

(event Collision|EventActorBeginOverlap
  (params (OtherActor :type Actor%20Object%20Reference)))

(event EventTick
  (params (DeltaSeconds :type Float%20%28single-precision%29)))

(event EventOnGameStateBegin
  (params (GameState :type BP%20Game%20State%20Character%20Selection%20Object%20Reference))
  (bind _foundwidgets (Class|WidgetBlueprintLibrary|GetAllWidgetswithInterface "/Game/LeagueOfWatch/Core/GameModes/DependOnLevel/CharacterSelection/BPI_CharacterSelectionEventListener.BPI_CharacterSelectionEventListener_C" false))
  (for _array_element _foundwidgets
    (Class|BPICharacterSelectionEventListener|OnGameStateBegin(Message) _array_element GameState)))

(event EventOnPlayerStateBegin
  (params (PlayerState :type BP%20Player%20State%20Character%20Selection%20Object%20Reference))
  (bind _foundwidgets (Class|WidgetBlueprintLibrary|GetAllWidgetswithInterface "/Game/LeagueOfWatch/Core/GameModes/DependOnLevel/CharacterSelection/BPI_CharacterSelectionEventListener.BPI_CharacterSelectionEventListener_C" false))
  (for _array_element _foundwidgets
    (Class|BPICharacterSelectionEventListener|OnPlayerStateBegin(Message) _array_element PlayerState)))

(event EventOnAllPlayersReady
  (bind _foundwidgets (Class|WidgetBlueprintLibrary|GetAllWidgetswithInterface "/Game/LeagueOfWatch/Core/GameModes/DependOnLevel/CharacterSelection/BPI_CharacterSelectionEventListener.BPI_CharacterSelectionEventListener_C" false))
  (for _array_element _foundwidgets
    (Class|BPICharacterSelectionEventListener|OnAllPlayersReady(Message) _array_element)))

(event EventOnLocalPlayerStateBegin
  (params (PlayerState :type BP%20Player%20State%20Character%20Selection%20Object%20Reference))
  (bind _foundwidgets (Class|WidgetBlueprintLibrary|GetAllWidgetswithInterface "/Game/LeagueOfWatch/Core/GameModes/DependOnLevel/CharacterSelection/BPI_CharacterSelectionEventListener.BPI_CharacterSelectionEventListener_C" false))
  (for _array_element _foundwidgets
    (Class|BPICharacterSelectionEventListener|OnLocalPlayerStateBegin(Message) _array_element PlayerState)))

(fn ConstructionScript)