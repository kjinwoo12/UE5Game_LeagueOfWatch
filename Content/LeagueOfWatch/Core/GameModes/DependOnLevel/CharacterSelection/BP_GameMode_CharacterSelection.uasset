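; Game mode for the character selection level that gathers connected players and splits them into Red and Blue teams.
; PostLogin registers up to ten controllers and fires the all-connected event when the count reaches two.
; That event runs placeholder team assignment (random, rerolled when a team has five, pending matchmaking-server data), then notifies BPI_CharacterSelectionEventListener actors.
; OnRequestTeamPlayers returns both team player-state lists to the requesting player.
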(event Custom|UpdatePlayerState
  (params (PlayerController :type BP%20Player%20Controller%20Character%20Selection%20Object%20Reference))
  (bind _playerstate (Variables|/Script/Engine.Controller|GetPlayerState PlayerController))
  (bind _blueteamplayerstate (Variables|Default|GetBlueTeamPlayerState))
  (bind _redteamplayerstate (Variables|Default|GetRedTeamPlayerState))
  (bind _returnvalue (Utilities|Array|Length _redteamplayerstate))
  (bind _returnvalue_2 (Utilities|Array|Length _blueteamplayerstate))
  ;[1 1 1] TEST CODE! #TODO: Change it to use the matchmaking server and get the information.
  (bind _asbp_player_state_character_selection (Utilities|Casting|CastToBP_PlayerState_CharacterSelection (Variables|/Script/Engine.Controller|GetPlayerState PlayerController)))
  (bind _output_get (Variables|/Game/LeagueOfWatch/Core/GameModes/DependOnLevel/CharacterSelection/BP_PlayerState_CharacterSelection.BP_PlayerState_CharacterSelection_C|SetTeam _asbp_player_state_character_selection (.OutItem (Utilities|Array|Random (Utilities|Array|MakeArray "NewEnumerator0" "NewEnumerator1"))) :!label _label))
  (switch Utilities|FlowControl|Switch|SwitchonETeam _output_get
    (:NewEnumerator0
      (if (>= _returnvalue 5)
        (goto _label)
        (else
          (Variables|/Game/LeagueOfWatch/Core/GameModes/DependOnLevel/CharacterSelection/BP_PlayerState_CharacterSelection.BP_PlayerState_CharacterSelection_C|SetUserName _asbp_player_state_character_selection (Utilities|Text|ToText(Integer) _returnvalue))
          (bind _asbp_player_state_character_selection_2 (Utilities|Casting|CastToBP_PlayerState_CharacterSelection _playerstate))
          (Utilities|Array|Add (Variables|Default|GetRedTeamPlayerState) _asbp_player_state_character_selection_2))))
    (:NewEnumerator1
      (if (>= _returnvalue_2 5)
        (goto _label)
        (else
          (Variables|/Game/LeagueOfWatch/Core/GameModes/DependOnLevel/CharacterSelection/BP_PlayerState_CharacterSelection.BP_PlayerState_CharacterSelection_C|SetUserName _asbp_player_state_character_selection (Utilities|Text|ToText(Integer) _returnvalue_2))
          (bind _asbp_player_state_character_selection_3 (Utilities|Casting|CastToBP_PlayerState_CharacterSelection _playerstate))
          (Utilities|Array|Add (Variables|Default|GetBlueTeamPlayerState) _asbp_player_state_character_selection_3))))))

(event Custom|OnAllPlayersConnected
  (Utilities|FlowControl|Sequence
    (:then_0
      (for _array_element (Variables|Default|GetConnectedPlayerController)
        (CallFunction|UpdatePlayerState _array_element)))
    (:then_1
      (bind _outactors (Actor|GetAllActorswithInterface "/Game/LeagueOfWatch/Core/GameModes/DependOnLevel/CharacterSelection/BPI_CharacterSelectionEventListener.BPI_CharacterSelectionEventListener_C"))
      (for _array_element_2 _outactors
        (Class|BPICharacterSelectionEventListener|OnAllPlayersConnected(Message) _array_element_2)))))

(event Custom|OnRequestTeamPlayers
  (params (Target%20Player :type BP%20Player%20Controller%20Character%20Selection%20Object%20Reference))
  (Default|OnResponseTeamPlayers Target%20Player (Variables|Default|GetRedTeamPlayerState) (Variables|Default|GetBlueTeamPlayerState)))

(event EventBeginPlay)

(event EventTick
  (params (DeltaSeconds :type Float%20%28single-precision%29)))

(event EventPostLogin
  (params (NewPlayer :type Player%20Controller%20Object%20Reference))
  (if (< (Utilities|Array|Length (Variables|Default|GetConnectedPlayerController)) 10)
    (bind _asbp_player_controller_character_selection (Utilities|Casting|CastToBP_PlayerController_CharacterSelection NewPlayer))
    (Utilities|Array|AddUnique (Variables|Default|GetConnectedPlayerController) _asbp_player_controller_character_selection)
    (if (== (Utilities|Array|Length (Variables|Default|GetConnectedPlayerController)) 2)
      (CallFunction|OnAllPlayersConnected))
    (else
      (|Logout NewPlayer))))

(fn ConstructionScript)