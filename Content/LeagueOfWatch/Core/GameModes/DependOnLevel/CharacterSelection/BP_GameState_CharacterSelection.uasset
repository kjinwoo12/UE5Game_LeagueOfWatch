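; Game state for the character selection level, holding the red and blue team rosters.
; On non-dedicated instances, BeginPlay notifies the first local player controller that the game state has begun.
; Initialize gives each player a random team, re-rolling when that team is full, and an indexed placeholder name.
; This assignment is marked temporary pending a matchmaking server, and StartSelectionTimer is an empty stub.
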(event Custom|InitializePlayer
  (params (Player :type Player%20State%20Object%20Reference))
  (bind _blueteamplayers (Variables|Default|GetBlueTeamPlayers))
  (bind _redteamplayers (Variables|Default|GetRedTeamPlayers))
  (bind _returnvalue (Utilities|Array|Length _redteamplayers))
  (bind _returnvalue_2 (Utilities|Array|Length _blueteamplayers))
  ;[1 1 1] %TEMP CODE% #TODO: Change it to use the matchmaking server and get the information.
  (bind _asbp_player_state_character_selection (Utilities|Casting|CastToBP_PlayerState_CharacterSelection Player))
  (bind _output_get (Variables|/Game/LeagueOfWatch/Core/GameModes/DependOnLevel/CharacterSelection/BP_PlayerState_CharacterSelection.BP_PlayerState_CharacterSelection_C|SetTeam _asbp_player_state_character_selection (.OutItem (Utilities|Array|Random (Utilities|Array|MakeArray "NewEnumerator0" "NewEnumerator1"))) :!label _label))
  (switch Utilities|FlowControl|Switch|SwitchonETeam _output_get
    (:NewEnumerator0
      (if (>= _returnvalue 5)
        (goto _label)
        (else
          (Variables|/Game/LeagueOfWatch/Core/GameModes/DependOnLevel/CharacterSelection/BP_PlayerState_CharacterSelection.BP_PlayerState_CharacterSelection_C|SetUserName _asbp_player_state_character_selection (Utilities|Text|ToText(String) (Utilities|String|Append "Red" (Utilities|String|ToString(Integer) _returnvalue))))
          (bind _asbp_player_state_character_selection_2 (Utilities|Casting|CastToBP_PlayerState_CharacterSelection Player))
          (Utilities|Array|Add (Variables|Default|GetRedTeamPlayers) _asbp_player_state_character_selection_2))))
    (:NewEnumerator1
      (if (>= _returnvalue_2 5)
        (goto _label)
        (else
          (Variables|/Game/LeagueOfWatch/Core/GameModes/DependOnLevel/CharacterSelection/BP_PlayerState_CharacterSelection.BP_PlayerState_CharacterSelection_C|SetUserName _asbp_player_state_character_selection (Utilities|Text|ToText(String) (Utilities|String|Append "Blue" (Utilities|String|ToString(Integer) _returnvalue_2))))
          (bind _asbp_player_state_character_selection_3 (Utilities|Casting|CastToBP_PlayerState_CharacterSelection Player))
          (Utilities|Array|Add (Variables|Default|GetBlueTeamPlayers) _asbp_player_state_character_selection_3))))))

(event Custom|Initialize
  (for _array_element (Variables|Default|GetPlayerArray)
    (CallFunction|InitializePlayer _array_element)))

(event EventBeginPlay
  (if (not (Networking|IsDedicatedServer))
    (bind _asbp_player_controller_character_selection (Utilities|Casting|CastToBP_PlayerController_CharacterSelection (Game|GetPlayerController 0)))
    (Default|OnGameStateBegin _asbp_player_controller_character_selection self)))

(event EventTick
  (params (DeltaSeconds :type Float%20%28single-precision%29)))

(fn ConstructionScript)

(fn StartSelectionTimer
  (params (Begin :type Float%20%28double-precision%29)))