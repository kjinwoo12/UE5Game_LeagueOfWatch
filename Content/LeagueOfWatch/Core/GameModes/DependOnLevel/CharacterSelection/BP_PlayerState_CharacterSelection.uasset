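; Player state for the character selection game mode that announces itself to the player controller and exposes its Team through a getter.
; On BeginPlay, outside dedicated servers, it casts its own player controller to the character selection controller and calls OnLocalPlayerStateBegin.
; If that cast fails, it treats itself as another player's state and calls OnPlayerStateBegin on player controller 0 instead.
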(event EventBeginPlay
  (if (not (Networking|IsDedicatedServer))
    (bind _asbp_player_controller_character_selection (Utilities|Casting|CastToBP_PlayerController_CharacterSelection (Game|GetPlayerController self))
      (:then
        (Default|OnLocalPlayerStateBegin _asbp_player_controller_character_selection self))
      (:CastFailed
        (bind _asbp_player_controller_character_selection_2 (Utilities|Casting|CastToBP_PlayerController_CharacterSelection (Game|GetPlayerController 0)))
        (Default|OnPlayerStateBegin _asbp_player_controller_character_selection_2 self)))))

(event EventTick
  (params (DeltaSeconds :type Float%20%28single-precision%29)))

(fn ConstructionScript)

(fn GetTeam
  (return (Variables|Default|GetTeam)))