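; In-game match GameMode that drives minion spawn timing, team start selection and the win or lose screen.
; After a short delay, a looping timer broadcasts minion spawn events to all BPI_IngameEvent actors.
; Nexus destruction compares the fallen team with player 0's to choose the result widget.
; It also spawns characters from CharacterInfo, caches each team's PlayerStart and forwards controller swaps to BP_PlayerController_Ingame.
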(event Custom|OnUpdateIngameLevelTimer
  (bind _outactors (Actor|GetAllActorswithInterface "/Game/LeagueOfWatch/Core/GameModes/DependOnLevel/Ingame/BPI_IngameEvent.BPI_IngameEvent_C"))
  (for _array_element _outactors
    (bind _asbpi_ingame_event (Utilities|Casting|CastToBPI_IngameEvent _array_element))
    (Default|OnSpawningMinionTimerEvent _asbpi_ingame_event)))

(event Custom|InitializeMinionTimer
  (bind _returnvalue (Utilities|Time|SetTimerbyEvent (delegate Custom|OnUpdateIngameLevelTimer) 5.0 true))
  (Variables|Handler|SetSpawnMinionHandle _returnvalue))

(event Custom|OnNexusDestroyed
  (params (Team :type ETeam%20Enum :default "NewEnumerator0"))
  (bind _team (Class|BPITeamSystem|GetTeam(Message) (Game|GetPlayerState 0)))
  (if (Utilities|Enum|Equal(Enum) _team Team)
    (bind _returnvalue (UserInterface|CreateWidget "/Game/LeagueOfWatch/Widgets/DependOnLevel/Ingame/WBP_IngameLevel_Lose.WBP_IngameLevel_Lose_C"))
    (UserInterface|Viewport|AddtoViewport _returnvalue 0)
    (else
      (bind _returnvalue_2 (UserInterface|CreateWidget "/Game/LeagueOfWatch/Widgets/DependOnLevel/Ingame/WBP_IngameLevel_Win.WBP_IngameLevel_Win_C"))
      (UserInterface|Viewport|AddtoViewport _returnvalue_2 0))))

(event EventBeginPlay
  (Development|PrintString "BP_GameMode_Ingame::BeginPlay")
  (Utilities|Time|SetTimerbyEvent (delegate Custom|InitializeMinionTimer) 1.0))

(event EventTick
  (params (DeltaSeconds :type Float%20%28single-precision%29)))

(event EventOnSwapPlayerControllers
  (params (OldPC :type Player%20Controller%20Object%20Reference) (NewPC :type Player%20Controller%20Object%20Reference))
  (Development|PrintString "BP_GameMode_Ingame::OnSwapPlayerControllers" true true "(R=0.000000,G=0.660000,B=1.000000,A=1.000000)" 2e+01)
  (bind _asbp_player_controller_ingame (Utilities|Casting|CastToBP_PlayerController_Ingame NewPC)
    (:then
      (Default|OnSwapPlayerController _asbp_player_controller_ingame OldPC))
    (:CastFailed
      (Development|PrintString "BP_GameMode_Ingame - Failed to cast BP_PlayerController_Ingame" true true "(R=0.000000,G=0.660000,B=1.000000,A=1.000000)" 2e+01))))

(fn ConstructionScript)

(fn SpawnCharacter
  (params (CharacterInfo :type S%20Playable%20Character%20Info%20Structure) (Team :type ETeam%20Enum :default "NewEnumerator0"))
  (bind _returnvalue (Game|SpawnActorfromClass (.CharacterReference (Utilities|Struct|BreakSPlayableCharacterInfo CharacterInfo)) (Math|Transform|MakeTransform "0, 0, 0" "0, 0, 0" "1.000000,1.000000,1.000000") "Undefined" "MultiplyWithRoot" 0 "/Game/LeagueOfWatch/Core/Characters/PlayableCharacter/Input/IMC_PlayableCharacter.IMC_PlayableCharacter" 0))
  (return _returnvalue))

(fn ChoosePlayerStart
  (params (Player :type Controller%20Object%20Reference))
  (bind _team (Class|BPITeamSystem|GetTeam(Message) Player))
  (switch Utilities|FlowControl|Switch|SwitchonETeam _team
    (:NewEnumerator0
      (if (!= (Variables|Default|GetRedTeamStart) 0)
        (return (Variables|Default|GetRedTeamStart))
        (else
          (bind _outactors (Actor|GetAllActorsOfClass "/Game/LeagueOfWatch/Core/GameModes/DependOnLevel/Ingame/BP_PlayerStart_Ingame.BP_PlayerStart_Ingame_C"))
          (for _array_element _outactors
            (bind _team_2 (Class|BPITeamSystem|GetTeam(Message) _array_element))
            (if (Utilities|Enum|Equal(Enum) _team_2 "NewEnumerator0")
              (Variables|Default|SetRedTeamStart _array_element)
              (return (Variables|Default|GetRedTeamStart))))
          (return 0))))
    (:NewEnumerator1
      (if (!= (Variables|Default|GetBlueTeamStart) 0)
        (return (Variables|Default|GetBlueTeamStart))
        (else
          (bind _outactors_2 (Actor|GetAllActorsOfClass "/Game/LeagueOfWatch/Core/GameModes/DependOnLevel/Ingame/BP_PlayerStart_Ingame.BP_PlayerStart_Ingame_C"))
          (for _array_element_2 _outactors_2
            (bind _team_3 (Class|BPITeamSystem|GetTeam(Message) _array_element_2))
            (if (Utilities|Enum|Equal(Enum) _team_3 "NewEnumerator1")
              (Variables|Default|SetBlueTeamStart _array_element_2)
              (return (Variables|Default|GetBlueTeamStart))))
          (return 0))))))