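; In-game player controller that carries each player's character selection into the match and gives them their pawn.
; On controller swap, it copies the confirmed character info and team from the outgoing character-selection controller, printing an error if the cast fails.
; When AllPlayersReady fires, it spawns the selected character class at a fixed location, adjusting for collisions, and possesses it.
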(event Custom|OnSwapPlayerController
  (params (Old%20PC :type Player%20Controller%20Object%20Reference))
  (bind _asbp_player_controller_character_selection (Utilities|Casting|CastToBP_PlayerController_CharacterSelection Old%20PC)
    (:then
      (Variables|Default|SetCharacterInfo (Variables|/Game/LeagueOfWatch/Core/GameModes/DependOnLevel/CharacterSelection/BP_PlayerController_CharacterSelection.BP_PlayerController_CharacterSelection_C|GetConfirmedCharacterInfo _asbp_player_controller_character_selection))
      (Variables|Default|SetTeam (Variables|/Game/LeagueOfWatch/Core/GameModes/DependOnLevel/CharacterSelection/BP_PlayerController_CharacterSelection.BP_PlayerController_CharacterSelection_C|GetTeam _asbp_player_controller_character_selection)))
    (:CastFailed
      (Development|PrintString "BP_PlayerController_Ingame::OnSwapPlayerController - Failed Cast to BP_PlayerController_CharacterSelection" true true "(R=0.000000,G=0.660000,B=1.000000,A=1.000000)" 2e+01))))

(event EventBeginPlay
  (Development|PrintString "BP_PlayerController_IngameLevel : BeginPlay"))

(event EventTick
  (params (DeltaSeconds :type Float%20%28single-precision%29)))

(event EventAllPlayersReady
  (bind _returnvalue (Game|SpawnActorfromClass (.CharacterReference (Utilities|Struct|BreakSPlayableCharacterInfo (Variables|Default|GetCharacterInfo))) (Math|Transform|MakeTransform "0.000000,0.000000,100.000000" "0, 0, 0" "1.000000,1.000000,1.000000") "AdjustIfPossibleButAlwaysSpawn" "MultiplyWithRoot" self 0))
  (Pawn|Possess _returnvalue)
  (Development|PrintString "BP_PlayerController_Ingame::BeginPlay && OnSwapPlayerController - Possessed"))

(fn ConstructionScript)