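; BP_Nexus is a team-owned Nexus game object that takes damage and can be destroyed.
; It sets HP to MaxHP on BeginPlay and subtracts incoming AnyDamage from it.
; When HP reaches zero or below, OnDied reports the owning Team to BP_GameMode_IngameLevel through OnNexusDestoyed.
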(event Custom|OnDied
  (bind _asbp_game_mode_ingame_level (Utilities|Casting|CastToBP_GameMode_IngameLevel (Game|GetGameMode)))
  (Default|OnNexusDestoyed _asbp_game_mode_ingame_level (Variables|Status|GetTeam)))

(event EventBeginPlay
  (Variables|Status|SetHP (Variables|Status|GetMaxHP)))

(event Collision|EventActorBeginOverlap
  (params (OtherActor :type Actor%20Object%20Reference)))

(event EventTick
  (params (DeltaSeconds :type Float%20%28single-precision%29)))

(event Game|Damage|EventAnyDamage
  (params (Damage :type Float%20%28single-precision%29) (DamageType :type Damage%20Type%20Object%20Reference) (InstigatedBy :type Controller%20Object%20Reference) (DamageCauser :type Actor%20Object%20Reference))
  (bind _output_get (Variables|Status|SetHP (- (Variables|Status|GetHP) Damage)))
  (if (<= _output_get 0.0)
    (CallFunction|OnDied)))

(fn ConstructionScript)