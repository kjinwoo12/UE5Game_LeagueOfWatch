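; Base projectile actor that flies toward a goal point and destroys itself on arrival.
; Each Tick it makes a swept move at Speed along the direction to GetGoal, re-querying the goal every frame.
; Once within ErrorRange, it calls the OnArrivedGoal event dispatcher before destroying itself.
; GetGoal returns the world origin here, apparently a placeholder for child classes to override.
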(event EventBeginPlay)

(event Collision|EventActorBeginOverlap
  (params (OtherActor :type Actor%20Object%20Reference)))

(event EventTick
  (params (DeltaSeconds :type Float%20%28single-precision%29))
  (bind _goal (CallFunction|GetGoal))
  (Class|Actor|AddActorWorldTransformKeepScale (Math|Transform|MakeTransform (* (Math|Vector|GetUnitDirection(Vector) (Transformation|GetActorLocation) _goal) (* DeltaSeconds (Variables|파라미터|GetSpeed))) "0, 0, 0" "1.000000,1.000000,1.000000") true false)
  (if (>= (Variables|파라미터|GetErrorRange) (Math|Vector|Distance(Vector) (Transformation|GetActorLocation) _goal))
    (Default|CallOnArrivedGoalEventDispatcher)
    (Actor|DestroyActor)))

(fn ConstructionScript)

(fn GetGoal
  (return "0, 0, 0"))