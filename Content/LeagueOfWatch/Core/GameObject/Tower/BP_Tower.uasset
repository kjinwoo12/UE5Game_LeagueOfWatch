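; BP_Tower is a team-owned, destructible tower that automatically fires guided projectiles at targets in its attack area.
; Its attack area component receives the tower's team and reports target updates; the tower locks onto the first target and attacks at once if off cooldown.
; Each shot starts a cooldown timer based on attack speed, whose completion fires again while the target stays valid.
; Incoming damage is reduced by armor, and the actor is destroyed when HP runs out.
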(event OnCoolTimeDone(BP_CoolTimerComponent_Attack)
  (Utilities|IsValid (Variables|Default|GetAttackTarget)
    (:Is%20Valid
      (CallFunction|DoAttack (Variables|Default|GetAttackTarget)))))

(event OnUpdaetAttackTargets(TowerAttackArea)
  (params (AttackTergets :type Array%20of%20Actor%20Object%20References))
  (if (== (Utilities|Array|Length AttackTergets) 0)
    (Variables|Default|SetAttackTarget 0)
    (else
      (bind _output_get (Variables|Default|SetAttackTarget (Utilities|Array|Get(acopy) AttackTergets)))
      (CallFunction|DoAttack _output_get))))

(event Custom|OnDied
  (Actor|DestroyActor))

(event EventBeginPlay
  (Variables|/Game/LeagueOfWatch/Core/GameObject/Tower/BP_TowerAttackArea.BP_TowerAttackArea_C|SetTeam (Variables|파라미터|GetTowerAttackArea) (Variables|파라미터|GetTeam)))

(event Game|Damage|EventAnyDamage
  (params (Damage :type Float%20%28single-precision%29) (DamageType :type Damage%20Type%20Object%20Reference) (InstigatedBy :type Controller%20Object%20Reference) (DamageCauser :type Actor%20Object%20Reference))
  (bind _returnvalue (Class|CombatFormulaFunctionLibrary|ArmoredDamageFormula Damage (.Armor (Utilities|Struct|BreakSStat (Variables|파라미터|GetStat)))))
  (bind _output_get (Variables|파라미터|SetHP (- (Variables|파라미터|GetHP) _returnvalue)))
  (if (<= _output_get 0.0)
    (CallFunction|OnDied)))

(fn ConstructionScript)

(fn DoAttack
  (params (AttackTarget :type Actor%20Object%20Reference))
  (bind _stat (Variables|파라미터|GetStat))
  (bind (_attackdamage _attackspeed) (Utilities|Struct|BreakSStat _stat))
  (if (<= (Variables|/Game/LeagueOfWatch/Core/CombatSystem/CoolTimer/BP_CoolTimerComponent.BP_CoolTimerComponent_C|GetCurrentCoolTime (Variables|Default|GetBP_CoolTimerComponent_Attack)) 0.0)
    (Game|SpawnActorfromClass "/Game/LeagueOfWatch/Core/GameObject/Tower/BP_GuidedProjectile_Tower.BP_GuidedProjectile_Tower_C" (Math|Transform|MakeTransform (Transformation|GetWorldLocation (Variables|Default|GetProjectileStartingPoint)) "0, 0, 0" "1.000000,1.000000,1.000000") "Undefined" 0 AttackTarget _attackdamage 3.6e+03 0)
    (Default|Start (Variables|Default|GetBP_CoolTimerComponent_Attack) (/ 1.0 _attackspeed))))

(fn GetTeam
  (return (Variables|파라미터|GetTeam)))