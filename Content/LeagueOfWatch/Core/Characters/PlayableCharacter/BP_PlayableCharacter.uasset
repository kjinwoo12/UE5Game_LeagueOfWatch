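; Player-controlled character base for LeagueOfWatch, handling Enhanced Input movement, look, jump and crouch, and exposing its team through GetTeam.
; On possession it adds the input mapping context if the controller has a local input subsystem.
; Otherwise it stores the controller in a RepNotify variable, whose OnRep adds the mapping context on the client, covering multiplayer where possession runs on the server.
; Debug prints trace possession and failures.
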(event Input|EnhancedActionEvents|EnhancedInputActionIA_Jump
  (params (ActionValue :type Boolean) (ElapsedSeconds :type Float%20%28double-precision%29) (TriggeredSeconds :type Float%20%28double-precision%29) (InputAction :type Input%20Action%20Object%20Reference :default "/Game/LeagueOfWatch/Core/Characters/PlayableCharacter/Input/IA_Jump.IA_Jump"))
  (:Triggered
    (Character|Jump))
  (:Completed
    (Character|StopJumping)))

(event Input|EnhancedActionEvents|EnhancedInputActionIA_Move
  (params (ActionValue :type Vector%202D%20Structure) (ElapsedSeconds :type Float%20%28double-precision%29) (TriggeredSeconds :type Float%20%28double-precision%29) (InputAction :type Input%20Action%20Object%20Reference :default "/Game/LeagueOfWatch/Core/Characters/PlayableCharacter/Input/IA_Move.IA_Move"))
  (Pawn|Input|AddMovementInput (Transformation|GetActorRightVector) (.x ActionValue) false)
  (Pawn|Input|AddMovementInput (Transformation|GetActorForwardVector) (.y ActionValue) false))

(event Input|EnhancedActionEvents|EnhancedInputActionIA_Look
  (params (ActionValue :type Vector%202D%20Structure) (ElapsedSeconds :type Float%20%28double-precision%29) (TriggeredSeconds :type Float%20%28double-precision%29) (InputAction :type Input%20Action%20Object%20Reference :default "/Game/LeagueOfWatch/Core/Characters/PlayableCharacter/Input/IA_Look.IA_Look"))
  (Pawn|Input|AddControllerYawInput (.x ActionValue))
  (Pawn|Input|AddControllerPitchInput (.y ActionValue)))

(event Input|EnhancedActionEvents|EnhancedInputActionIA_Crouch
  (params (ActionValue :type Boolean) (ElapsedSeconds :type Float%20%28double-precision%29) (TriggeredSeconds :type Float%20%28double-precision%29) (InputAction :type Input%20Action%20Object%20Reference :default "/Game/LeagueOfWatch/Core/Characters/PlayableCharacter/Input/IA_Crouch.IA_Crouch"))
  (if ActionValue
    (Character|Crouch)
    (else
      (Character|UnCrouch))))

(event Collision|EventActorBeginOverlap
  (params (OtherActor :type Actor%20Object%20Reference)))

(event EventTick
  (params (DeltaSeconds :type Float%20%28single-precision%29)))

(event EventPossessed
  (params (NewController :type Controller%20Object%20Reference))
  (Development|PrintString "BP_PlayableCharacter::Possessed " true true "(R=0.000000,G=0.660000,B=1.000000,A=1.000000)" 2e+01)
  (bind _as플레이어_컨트롤러 (Utilities|Casting|CastToPlayerController NewController)
    (:then
      (Utilities|IsValid (PlayerController|LocalPlayerSubsystems|GetEnhancedInputLocalPlayerSubsystem _as플레이어_컨트롤러)
        (:Is%20Valid
          (Input|AddMappingContext (PlayerController|LocalPlayerSubsystems|GetEnhancedInputLocalPlayerSubsystem _as플레이어_컨트롤러) "/Game/LeagueOfWatch/Core/Characters/PlayableCharacter/Input/IMC_PlayableCharacter.IMC_PlayableCharacter" 0 "(bIgnoreAllPressedKeysUntilRelease=True,bForceImmediately=False,bNotifyUserSettings=False)"))
        (:Is%20Not%20Valid
          (Variables|Default|SetPlayerControllerForMultiplay _as플레이어_컨트롤러))))
    (:CastFailed
      (Development|PrintString "BP_PlayableCharacter::Possessed - Failed Cast to PlayerController" true true "(R=0.000000,G=0.660000,B=1.000000,A=1.000000)" 2e+01))))

(fn ConstructionScript)

(fn OnRepPlayerControllerforMultiplay
  (bind _playercontrollerformultiplay (Variables|Default|GetPlayerControllerForMultiplay))
  (bind _returnvalue (PlayerController|LocalPlayerSubsystems|GetEnhancedInputLocalPlayerSubsystem _playercontrollerformultiplay))
  (Utilities|IsValid _returnvalue
    (:Is%20Valid
      (Input|AddMappingContext _returnvalue (Variables|Default|GetMappingContext) 0 "(bIgnoreAllPressedKeysUntilRelease=True,bForceImmediately=False,bNotifyUserSettings=False)"))
    (:Is%20Not%20Valid
      (Development|PrintString "BP_PlayableCharacter::OnRep_PlayerCOntrollerForMultiplay - Invalid EnhancedInputLocalPlayerSubsystem" true true "(R=0.000000,G=0.660000,B=1.000000,A=1.000000)" 2e+01))))

(fn GetTeam
  (return (Variables|Default|GetTeam)))