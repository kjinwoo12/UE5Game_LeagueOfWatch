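; Tracer's playable character Blueprint, a child class that adds animation layer setup and a possession debug UI.
; On BeginPlay it links feminine or default unarmed animation layers to the mesh, based on a cosmetic gameplay tag.
; Possession and unpossession call ClientRPC-named events that create and remove a debug widget in the viewport.
; The primary attack input event is an empty stub.
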(event Custom|ClientRPCOnPossessed
  (bind _returnvalue (UserInterface|CreateWidget "/Game/LeagueOfWatch/Widgets/Debug/WBP_Debug_playableCharacter.WBP_Debug_playableCharacter_C"))
  (bind _output_get (Variables|Default|SetAddedWidget _returnvalue))
  (UserInterface|Viewport|AddtoViewport _output_get 0))

(event Custom|ClientRPCOnUnpossessed
  (Widget|RemovefromParent (Variables|Default|GetAddedWidget)))

(event Input|EnhancedActionEvents|EnhancedInputActionIA_PrimaryAttack
  (params (ActionValue :type Boolean) (ElapsedSeconds :type Float%20%28double-precision%29) (TriggeredSeconds :type Float%20%28double-precision%29) (InputAction :type Input%20Action%20Object%20Reference :default "/Game/LeagueOfWatch/Core/Characters/PlayableCharacter/Input/IA_PrimaryAttack.IA_PrimaryAttack")))

(event EventBeginPlay
  (|CallParentFunction)
  (CallFunction|InitAnimClassLayers))

(event Collision|EventActorBeginOverlap
  (params (OtherActor :type Actor%20Object%20Reference))
  (|CallParentFunction OtherActor) ; 지금 이 노드는 비활성 상태입니다. \n핀을 끌어서 다른 노드를 연결하면 활성화됩니다.
)

(event EventTick
  (params (DeltaSeconds :type Float%20%28single-precision%29))
  (|CallParentFunction DeltaSeconds) ; 지금 이 노드는 비활성 상태입니다. \n핀을 끌어서 다른 노드를 연결하면 활성화됩니다.
)

(event EventPossessed
  (params (NewController :type Controller%20Object%20Reference))
  (|CallParentFunction NewController)
  (CallFunction|ClientRPConPossessed))

(event EventUnpossessed
  (params (OldController :type Controller%20Object%20Reference))
  (|CallParentFunction OldController)
  (CallFunction|ClientRPConUnpossessed))

(fn ConstructionScript
  (|CallParentFunction))

(fn InitAnimClassLayers
  (if (Utilities|Array|ContainsItem (.gameplaytags (Variables|Default|GetGameplayTagContainer)) "(TagName=\"Cosmetic.AnimationStyle.Female\")")
    (Components|SkeletalMesh|AnimationBlueprintLinking|LinkAnimClassLayers (Variables|Character|GetMesh) "/Game/Characters/Mannequin/Animations/Locomotion/Unarmed/ABP_UnarmedAnimLayers_Feminine.ABP_UnarmedAnimLayers_Feminine_C")
    (else
      (Components|SkeletalMesh|AnimationBlueprintLinking|LinkAnimClassLayers (Variables|Character|GetMesh) "/Game/Characters/Mannequin/Animations/Locomotion/Unarmed/ABP_UnarmedAnimLayers.ABP_UnarmedAnimLayers_C"))))