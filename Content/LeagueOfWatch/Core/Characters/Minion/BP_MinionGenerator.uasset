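; BP_MinionGenerator is an actor that spawns groups of minions for League of Watch.
; Each OnPrepareMinionGroupEvent increments SpawnCount and picks the cannon minion group on every third count, otherwise the default group.
; SpawnMinionGroup loops over the chosen class array, with a SpawnInterval Delay before each spawn node, adjusting for collisions but always spawning.
; BeginPlay and Tick are empty, and nothing in this Blueprint calls the prepare event.
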(event Custom|SpawnMinionGroup
  (params (MinionClass :type Array%20of%20BP%20Minion%20Class%20References))
  (for _array_element MinionClass
    (Utilities|FlowControl|Delay (Variables|Params|GetSpawnInterval))
    (Game|SpawnActorfromClass _array_element (Math|Transform|MakeTransform "0, 0, 0" "0, 0, 0" "1.000000,1.000000,1.000000") "AdjustIfPossibleButAlwaysSpawn" 0 0)))

(event EventBeginPlay)

(event Collision|EventActorBeginOverlap
  (params (OtherActor :type Actor%20Object%20Reference)))

(event EventTick
  (params (DeltaSeconds :type Float%20%28single-precision%29)))

(event EventOnPrepareMinionGroupEvent
  (bind _result (Math|Integer|IncrementInt (Variables|Default|GetSpawnCount))
    (:%20%20
      (if (== (Math|Integer|%(Integer) _result 3) 0)
        (CallFunction|SpawnMinionGroup (Variables|Const|GetCannonMinionGroup))
        (else
          (CallFunction|SpawnMinionGroup (Variables|Const|GetDefaultMinionGroup)))))))

(fn ConstructionScript)