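; BP_Minion is a team-based minion character that follows patrol points, attacks targets and dies when HP runs out.
; Patrol point arrivals are forwarded to AIC_Minion, and construction hides one of two meshes to show the team.
; DoAttack checks range and a cooldown timer driven by attack speed, then stops movement and spawns a guided projectile.
; Incoming damage passes through the damage type's defense formula against the minion's stats before reducing HP.
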(event Custom|OnArrivedToPatrolPoint
  (params (NextPatrolPoint :type BP%20Minion%20Patrol%20Point%20Object%20Reference))
  (bind _output_get (Variables|Params|SetPatrolPoint NextPatrolPoint))
  (bind _asaic_minion (Utilities|Casting|CastToAIC_Minion (Pawn|GetController))
    (:then
      (Default|OnChangedMinionPatrolPoint _asaic_minion _output_get))
    (:CastFailed
      (Development|PrintString "BP_Minion::OnArrivedPatrolPoint - Failed to convert Controller to AIC_Minion"))))

(event Custom|OnDied
  (Actor|DestroyActor))

(event EventBeginPlay)

(event Collision|EventActorBeginOverlap
  (params (OtherActor :type Actor%20Object%20Reference)))

(event EventTick
  (params (DeltaSeconds :type Float%20%28single-precision%29)))

(event Game|Damage|EventAnyDamage
  (params (Damage :type Float%20%28single-precision%29) (DamageType :type Damage%20Type%20Object%20Reference) (InstigatedBy :type Controller%20Object%20Reference) (DamageCauser :type Actor%20Object%20Reference))
  ;[0.8021 1 0.8832] Checkout `Core/DamageTypes`
  (bind _actualdamage (Class|BPIDamageType|DamageDefenseFormula(Message) DamageType Damage (Variables|Status|GetStat)))
  (bind _output_get (Variables|Status|SetHP (- (Variables|Status|GetHP) _actualdamage)))
  (if (<= _output_get 0.0)
    (CallFunction|OnDied)))

(fn ConstructionScript
  (switch Utilities|FlowControl|Switch|SwitchonETeam (Variables|Params|GetTeam)
    (:NewEnumerator0
      (Rendering|SetVisibility (Variables|Default|GetCube1) false false))
    (:NewEnumerator1
      (Rendering|SetVisibility (Variables|Default|GetSphere) false false))))

(fn ApplyAttackDamage
  (params (DamagedActor :type Actor%20Object%20Reference))
  (Game|Damage|ApplyDamage DamagedActor (.AttackDamage (Utilities|Struct|BreakSStat (Variables|Status|GetStat))) (Pawn|GetController) self "/Game/LeagueOfWatch/Core/CombatSystem/DamageTypes/BP_DamageType_AttackDamage.BP_DamageType_AttackDamage_C"))

(fn IsinAttackRange
  (params (TargetActor :type Actor%20Object%20Reference))
  (return (<= (Transformation|GetDistanceTo TargetActor) (Variables|Status|GetAttackRange))))

(fn DoAttack
  (params (TargetActor :type Actor%20Object%20Reference))
  (bind _stat (Variables|Status|GetStat))
  (bind (_attackdamage _attackspeed) (Utilities|Struct|BreakSStat _stat))
  (bind _issuccess (CallFunction|IsinAttackRange TargetActor))
  (if (and _issuccess (Default|IsOffCool (Variables|Default|GetBP_CoolTimerComponent_Attack)))
    (Class|NavMovementComponent|StopActiveMovement (Variables|Character|GetCharacterMovement))
    (Game|SpawnActorfromClass "/Game/LeagueOfWatch/Core/Characters/Minion/BP_GuidedProjectile_Minion.BP_GuidedProjectile_Minion_C" (Transformation|GetActorTransform) "Undefined" 0 TargetActor _attackdamage 5e+02 0)
    (Default|Start (Variables|Default|GetBP_CoolTimerComponent_Attack) (/ 1.0 _attackspeed))))

(fn GetTeam
  (return (Variables|Params|GetTeam)))